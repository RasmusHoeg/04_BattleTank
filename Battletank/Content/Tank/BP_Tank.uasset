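; BP_Tank is the player-controllable tank Blueprint that handles camera aiming and firing input.
; On BeginPlay it registers its Barrel and Turret components through SetBarrelReference and SetTurretReference.
; Aim axes rotate the AzimuthGimbal in yaw and the Elevation component in pitch, scaled by delta time for frame-rate independence.
; The Fire action calls Fire, while tick, overlap and construction logic are empty.
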(event `self.ReceiveBeginPlay`
  (`self.SetBarrelReference` (`self.Barrel`))
  (`self.SetTurretReference` (`self.Turret`)))

(event `InputAxis|Aim Azimuth`
  (params (AxisValue :type "Float (single-precision)"))
  ;[1 1 1] Input bindings
  (`SceneComponent.K2_AddLocalRotation` (`self.Azimuth Gimbal`) (`KismetMathLibrary.MakeRotator` 0.0 0.0 (* AxisValue (`GameplayStatics.GetWorldDeltaSeconds`) 100.0)) false false))

(event `InputAxis|Aim Elevation`
  (params (AxisValue :type "Float (single-precision)"))
  ;[1 1 1] Input bindings
  (`SceneComponent.K2_AddLocalRotation` (`self.Elevation`) (`KismetMathLibrary.MakeRotator` 0.0 (* (`GameplayStatics.GetWorldDeltaSeconds`) AxisValue 100.0)) false false))

(event `InputAction|Fire`
  (params (Key :type "Key Structure" :default "AnyKey"))
  ;[1 1 1] Input bindings
  (:`Pressed`
    (`self.Fire`)))

(fn `UserConstructionScript`)